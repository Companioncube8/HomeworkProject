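; BP_Turret is a turret actor Blueprint that handles the visual and physical cleanup when the turret explodes.
; On BeginPlay it binds a handler to the OnExplode event dispatcher.
; The handler hides the barrel and base meshes, disables their collision and sets a short lifespan, so the actor is destroyed after a brief delay.
; Tick, overlap and the construction script do nothing.
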(event `self.ReceiveBeginPlay`
  (add `self.OnExplode` (delegate `OnExplodeEvent`)))

(event `OnExplodeEvent`
  (`SceneComponent.SetVisibility` (`self.BarellMesh`) false false)
  (`SceneComponent.SetVisibility` (`self.TurretBaseMesh`) false false)
  (`PrimitiveComponent.SetCollisionEnabled` (`self.BarellMesh`) "NoCollision")
  (`PrimitiveComponent.SetCollisionEnabled` (`self.TurretBaseMesh`) "NoCollision")
  (`self.SetLifeSpan` 2.0))

(fn `UserConstructionScript`)